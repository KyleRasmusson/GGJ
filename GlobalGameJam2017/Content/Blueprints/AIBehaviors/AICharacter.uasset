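; AI character Blueprint that switches between normal and alerted states based on the player pawn's proximity.
; A sphere overlap triggers alert on entry and normal on exit, toggling a flag, swapping the mesh material and doubling or halving walk speed.
; BeginPlay applies the normal state, so walk speed starts at half its default.
; A Delay on Tick periodically spawns a "Sound" particle emitter at its location as a movement ping.
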(event `self.ReceiveBeginPlay`
  (`self.IsNormal`))

(event `self.Sphere.OnComponentBeginOverlap`
  (params (OverlappedComponent :type "PrimitiveComponent Object Reference") (OtherActor :type "Actor Object Reference") (OtherComp :type "PrimitiveComponent Object Reference") (OtherBodyIndex :type Integer) (bFromSweep :type Boolean) (SweepResult :type "HitResult Structure (by ref)"))
  (if (== OtherActor (`GameplayStatics.GetPlayerPawn` 0))
    (`self.isAlert`)))

(event `self.Sphere.OnComponentEndOverlap`
  (params (OverlappedComponent :type "PrimitiveComponent Object Reference") (OtherActor :type "Actor Object Reference") (OtherComp :type "PrimitiveComponent Object Reference") (OtherBodyIndex :type Integer))
  (if (== OtherActor (`GameplayStatics.GetPlayerPawn` 0))
    (`self.IsNormal`)))

(event `self.ReceiveTick`
  (params (DeltaSeconds :type "Float (single-precision)"))
  (`KismetSystemLibrary.Delay` 0.8)
  (`self.MovePing`))

(fn `isAlert`
  (bind _charactermovement (`self.CharacterMovement`))
  (set `self.isAlerted` true)
  (set `CharacterMovementComponent.MaxWalkSpeed` (* (`CharacterMovementComponent.MaxWalkSpeed` _charactermovement) 2.0) _charactermovement)
  (`PrimitiveComponent.SetMaterial` (`self.Mesh`) 0 "/Game/StarterContent/Materials/M_Brick_Clay_New.M_Brick_Clay_New"))

(fn `IsNormal`
  (bind _charactermovement (`self.CharacterMovement`))
  (set `self.isAlerted` false)
  (set `CharacterMovementComponent.MaxWalkSpeed` (* (`CharacterMovementComponent.MaxWalkSpeed` _charactermovement) 0.5) _charactermovement)
  (`PrimitiveComponent.SetMaterial` (`self.Mesh`) 0 "/Game/Mannequin/Character/Materials/M_UE4Man_Body.M_UE4Man_Body"))

(fn `MovePing`
  (`GameplayStatics.SpawnEmitterAtLocation` "/Game/ParticleEffect/Sound.Sound" (`self.K2_GetActorLocation`)))

(fn `UserConstructionScript`)