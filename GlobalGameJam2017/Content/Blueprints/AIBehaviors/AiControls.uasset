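; AI controller that walks an AICharacter along a chain of linked patrol nodes and chases the player when alerted.
; BeginPlay caches the pawn and starts toward its DesiredNode.
; Tick chases player 0 while IsAlerted; otherwise, when move status differs from DesiredStatus, it advances to NextNode and targets itself.
; It then nudges yaw via a lerp in LookAround and waits a random delay before moving to the node.
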(event `self.ReceiveBeginPlay`
  (bind _asaicharacter (cast `/Game/Blueprints/AIBehaviors/AICharacter` (`self.K2_GetPawn`)))
  (bind _output_get (set `self.Stored Pawn` _asaicharacter))
  (`self.MoveToActor` (`/Game/Blueprints/AIBehaviors/AICharacter.DesiredNode` _output_get) 20.0))

(event `self.ReceiveTick`
  (params (DeltaSeconds :type "Float (single-precision)"))
  (bind _stored_pawn (`self.Stored Pawn`))
  (if (`/Game/Blueprints/AIBehaviors/AICharacter.isAlerted` (`self.Stored Pawn`))
    (`self.MoveToActor` (`GameplayStatics.GetPlayerPawn` 0) 0.0)
    (elif (!= (`self.GetMoveStatus`) (`self.DesiredStatus`))
      (bind _output_get (set `/Game/Blueprints/AIBehaviors/AICharacter.DesiredNode` (`/Game/Blueprints/AIBehaviors/PathNode.NextNode` (`/Game/Blueprints/AIBehaviors/AICharacter.DesiredNode` _stored_pawn)) _stored_pawn))
      (`self.MoveToActor` self 20.0)
      (`self.LookAround`)
      (`KismetSystemLibrary.Delay` (`KismetMathLibrary.RandomFloatInRange` 0.5 3.0))
      (`self.MoveToActor` _output_get 20.0))))

(fn `LookAround`
  (bind _returnvalue (`self.K2_GetActorRotation` (`self.K2_GetPawn`)))
  (`self.K2_SetActorRotation` (`self.K2_GetPawn`) (`KismetMathLibrary.RLerp` _returnvalue (`KismetMathLibrary.MakeRotator` 0.0 0.0 (+ (.yaw _returnvalue) 45.0)) 0.075) false))

(fn `UserConstructionScript`)