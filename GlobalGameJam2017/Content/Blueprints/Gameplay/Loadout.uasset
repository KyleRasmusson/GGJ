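; Loadout component for the top-down character that spawns traps from three slots (Q, E, Space).
; Each slot checks its cooldown and optional on-map limit, spawns its trap class, increments the count, then starts a timer that re-arms it.
; A validity macro skips the timer for non-positive cooldowns.
; A transform helper selects between the cursor hit location and a fixed-height point ahead of the owner's TrapLocation.
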(event `Q Traps`
  (if (`self.Q Trap Cooled Down?`)
    (if (`self.Q Traps number important?`)
      (if (< (`self.Q Traps on map`) (`self.Q Trap Max`))
        (`|SpawnActorFromClass` (`self.Q Trap`) (`self.Spawn Transform` (`self.Q Use Mouse Loc?`)) "Undefined" "OverrideRootScale" :!label _label)
        (bind _result (`/Engine/EditorBlueprintResources/StandardMacros.IncrementInt` (`self.Q Traps on map`))
          (:`  `
            (set `self.Q Traps on map` _result)
            (set `self.Q Trap Cooled Down?` false)
            (`self.Time is Valid?` (`self.Q Trap Cooldown time`)
              (:`true`
                (bind _returnvalue (`KismetSystemLibrary.K2_SetTimerDelegate` (delegate `Q Trap Cooldown`) (`self.Q Trap Cooldown time`)))
                (set `self.Q Trap Timer` _returnvalue))
              (:`false`
                (`self.Q Trap Cooldown`))))))
      (else
        (goto _label)))))

(event `Q Trap Cooldown`
  (set `self.Q Trap Cooled Down?` true)
  (`KismetSystemLibrary.K2_ClearAndInvalidateTimerHandle` (`self.Q Trap Timer`)))

(event `E Traps`
  (bind _e_trap_cooldown_time (`self.E Trap Cooldown time`))
  (if (`self.E Trap Cooled Down?`)
    (if (`self.E Traps number important?`)
      (if (< (`self.E Traps on map`) (`self.E Traps Max`))
        (`|SpawnActorFromClass` (`self.E Trap`) (`self.Spawn Transform` (`self.E Use Mouse Loc?`)) "Undefined" "OverrideRootScale" :!label _label_2)
        (bind _result (`/Engine/EditorBlueprintResources/StandardMacros.IncrementInt` (`self.E Traps on map`))
          (:`  `
            (set `self.E Traps on map` _result)
            (set `self.E Trap Cooled Down?` false)
            (`self.Time is Valid?` _e_trap_cooldown_time
              (:`true`
                (bind _returnvalue (`KismetSystemLibrary.K2_SetTimerDelegate` (delegate `E Trap Cooldown`) _e_trap_cooldown_time))
                (set `self.E Trap Timer` _returnvalue))
              (:`false`
                (`self.E Trap Cooldown`))))))
      (else
        (goto _label_2)))))

(event `E Trap Cooldown`
  (set `self.E Trap Cooled Down?` true)
  (`KismetSystemLibrary.K2_ClearAndInvalidateTimerHandle` (`self.E Trap Timer`)))

(event `Space Traps`
  (bind _space_trap_cooldown_time (`self.Space Trap Cooldown time`))
  (if (`self.Space Traps Cooled Down?`)
    (if (`self.Space Traps number important?`)
      (if (< (`self.Space Traps on map`) (`self.Space Traps Max`))
        (`|SpawnActorFromClass` (`self.Space Trap`) (`self.Spawn Transform` (`self.Space Use Mouse Loc?`)) "Undefined" "OverrideRootScale" :!label _label_3)
        (bind _result (`/Engine/EditorBlueprintResources/StandardMacros.IncrementInt` (`self.Space Traps on map`))
          (:`  `
            (set `self.Space Traps on map` _result)
            (set `self.Space Traps Cooled Down?` false)
            (`self.Time is Valid?` _space_trap_cooldown_time
              (:`true`
                (bind _returnvalue (`KismetSystemLibrary.K2_SetTimerDelegate` (delegate `Space Cooldown`) _space_trap_cooldown_time))
                (set `self.Space Trap Timer` _returnvalue))
              (:`false`
                (`self.Space Cooldown`))))))
      (else
        (goto _label_3)))))

(event `Space Cooldown`
  (set `self.Space Traps Cooled Down?` true)
  (`KismetSystemLibrary.K2_ClearAndInvalidateTimerHandle` (`self.Space Trap Timer`)))