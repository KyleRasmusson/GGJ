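; Trap actor that deals a fixed, heavy hit of damage to enemies that overlap it.
; On overlap, it looks for an Enemy_Health component on the other actor, calls Damage on it and spawns an explosion effect and sound at its own location.
; The trap is not destroyed afterward.
; Tick draws a long-lived debug sphere matching the Sphere component's radius every frame.
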(event `self.ReceiveActorBeginOverlap`
  (params (OtherActor :type "Actor Object Reference"))
  (bind _returnvalue (`self.GetComponentByClass` OtherActor "/Game/Blueprints/Gameplay/Enemy_Health.Enemy_Health_C"))
  (`/Engine/EditorBlueprintResources/StandardMacros.IsValid` _returnvalue
    (:`Is Valid`
      (`/Game/Blueprints/Gameplay/Health.Damage` _returnvalue 100)
      (`GameplayStatics.SpawnEmitterAtLocation` "/Game/StarterContent/Particles/P_Explosion.P_Explosion" (`self.K2_GetActorLocation`))
      (`GameplayStatics.SpawnSoundAtLocation` "/Game/StarterContent/Audio/Explosion02.Explosion02" (`self.K2_GetActorLocation`)))))

(event `self.ReceiveTick`
  (params (DeltaSeconds :type "Float (single-precision)"))
  (`KismetSystemLibrary.DrawDebugSphere` (`self.K2_GetActorLocation`) (`SphereComponent.SphereRadius` (`self.Sphere`)) 12 (struct :`R` 0.234243 :`G` 1.0 :`A` 1.0) 20.0 2.0))

(fn `UserConstructionScript`)