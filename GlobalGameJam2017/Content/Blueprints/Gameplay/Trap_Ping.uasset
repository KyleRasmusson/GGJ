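; Trap actor that kills or heavily damages any enemy that overlaps it, then destroys itself.
; On overlap with an actor that has an Enemy_Health component, it applies fixed damage and calls Particles to spawn fire and a collapse sound at its location.
; It also decrements ETrapsOnMap on the player character's Loadout, writes the result to ETrapsMax, and prints a debug message.
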(event `self.ReceiveActorBeginOverlap`
  (params (OtherActor :type "Actor Object Reference"))
  (bind _returnvalue (`self.GetComponentByClass` OtherActor "/Game/Blueprints/Gameplay/Enemy_Health.Enemy_Health_C"))
  (bind _loadout (`/Game/TopDownBP/Blueprints/TopDownCharacter.Loadout` (cast `/Game/TopDownBP/Blueprints/TopDownCharacter` (`GameplayStatics.GetPlayerPawn` 0) :!pure true)))
  (`/Engine/EditorBlueprintResources/StandardMacros.IsValid` _returnvalue
    (:`Is Valid`
      (`/Game/Blueprints/Gameplay/Health.Damage` _returnvalue 100)
      (`self.Particles`)
      (bind _result (`/Engine/EditorBlueprintResources/StandardMacros.DecrementInt` (`/Game/Blueprints/Gameplay/Loadout.E Traps on map` _loadout))
        (:`  `
          (set `/Game/Blueprints/Gameplay/Loadout.E Traps Max` _result _loadout)
          (`KismetSystemLibrary.PrintString` "KILL PING!")
          (`self.K2_DestroyActor`))))))

(fn `UserConstructionScript`)