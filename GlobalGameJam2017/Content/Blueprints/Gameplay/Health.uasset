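; Health component that tracks damage taken by its owning actor and destroys that actor when health runs out.
; BeginPlay stores the initial Health as StartHealth, and the Damage event subtracts the incoming amount from Health.
; At zero or below, it sets Dead and calls Death, which spawns an explosion particle and sound at the owner's location, then destroys the owner.
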(event `self.ReceiveBeginPlay`
  (set `self.StartHealth` (`self.Health`)))

(event `Damage`
  (params (Damage :type Integer))
  (bind _output_get (set `self.Health` (- (`self.Health`) Damage)))
  (if (<= _output_get 0)
    (set `self.Dead` true)
    (`self.Death`)))

(fn `Death`
  (bind _returnvalue (`Actor.K2_GetActorLocation` (`self.GetOwner`)))
  (`GameplayStatics.SpawnEmitterAtLocation` "/Game/StarterContent/Particles/P_Explosion.P_Explosion" _returnvalue)
  (`GameplayStatics.SpawnSoundAtLocation` "/Game/StarterContent/Audio/Explosion02.Explosion02" _returnvalue)
  (`Actor.K2_DestroyActor` (`self.GetOwner`)))